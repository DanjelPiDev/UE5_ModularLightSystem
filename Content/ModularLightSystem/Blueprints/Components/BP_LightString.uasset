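; Light string from the modular light system that pairs a cable with lights spawned along a spline.
; On BeginPlay (marked WIP), it matches cable length to the spline and spawns evenly spaced lights, defaulting to BP_Light, with shared appearance, flicker and gradient settings.
; Interact toggles every light, though CanInteract always returns false.
; Tick divides the current cable length by root X scale every frame, so non-unit scales compound.
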(event EventBeginPlay
  ;[0.15 0.01719 0 0.5] WIP
  (CallFunction|SpawnLightsonSpline))

(event EventTick
  (params (DeltaSeconds :type Float%20%28single-precision%29))
  (bind _cable (Variables|Default|GetCable))
  (Variables|/Script/CableComponent.CableComponent|SetCableLength _cable (/ (Variables|/Script/CableComponent.CableComponent|GetCableLength _cable) (.X (Math|Vector|BreakVector (Transformation|GetWorldScale (Variables|Default|GetDefaultSceneRoot)))))))

(event EventInteract
  (params (Caller :type Actor%20Object%20Reference) (ActiveState :type Boolean))
  (for _array_element (Variables|Default|GetLights)
    (Default|ToggleLight _array_element (not (Variables|/Game/ModularLightSystem/Blueprints/Components/BP_Light.BP_Light_C|GetIsActive? _array_element)))))

(fn ConstructionScript
  (Collision|SetCollisionEnabled (Variables|Default|GetCable) (Variables|CableSettings|GetCableCollision))
  (Variables|/Script/CableComponent.CableComponent|SetbEnableStiffness (Variables|Default|GetCable) (Variables|CableSettings|GetUseStiffness?)))

(fn SpawnLightsonSpline
  (Variables|/Script/CableComponent.CableComponent|SetCableLength (Variables|Default|GetCable) (Spline|GetSplineLength (Variables|Default|GetSpline)))
  (if (> (Variables|LightStringSettings|GetNumOfLights) 0)
    (for _index (range 1 (Variables|LightStringSettings|GetNumOfLights))
      (if (Utilities|IsValidClass (Variables|LightStringSettings|GetSpawnSpecificLightBP))
        _
        (else
          (Variables|LightStringSettings|SetSpawnSpecificLightBP "/Game/ModularLightSystem/Blueprints/Components/BP_Light.BP_Light_C")))
      (bind _returnvalue (Game|SpawnActorfromClass (Variables|LightStringSettings|GetSpawnSpecificLightBP) (Math|Conversions|ToTransform(Vector) (Spline|GetLocationatDistanceAlongSpline (Variables|Default|GetSpline) (* _index (/ (Spline|GetSplineLength (Variables|Default|GetSpline)) (+ (Variables|LightStringSettings|GetNumOfLights) 1))) "World")) "AlwaysSpawn" "MultiplyWithRoot" 0 0))
      (bind _output_get (LocalVariables|SetCurrentLight _returnvalue))
      (Default|UpdateGeneralLightSettings _output_get)
      (Class|LocalLightComponent|SetIntensityUnits (Variables|/Game/ModularLightSystem/Blueprints/Components/BP_Light.BP_Light_C|GetPointLight (LocalVariables|GetCurrentLight)) "Lumens")
      (Rendering|Components|Light|SetIntensity (Variables|/Game/ModularLightSystem/Blueprints/Components/BP_Light.BP_Light_C|GetPointLight (LocalVariables|GetCurrentLight)) (Variables|LightStringSettings|GetLightIntensity))
      (Class|PointLightComponent|SetSourceRadius (Variables|/Game/ModularLightSystem/Blueprints/Components/BP_Light.BP_Light_C|GetPointLight (LocalVariables|GetCurrentLight)) (Variables|LightStringSettings|GetLightRadius))
      (Rendering|Components|Light|SetLightColor (Variables|/Game/ModularLightSystem/Blueprints/Components/BP_Light.BP_Light_C|GetPointLight (LocalVariables|GetCurrentLight)) (Variables|LightStringSettings|GetLightColor) true)
      (Transformation|SetActorLocation (LocalVariables|GetCurrentLight) (Spline|GetLocationatDistanceAlongSpline (Variables|Default|GetSpline) (* _index (/ (Spline|GetSplineLength (Variables|Default|GetSpline)) (+ (Variables|LightStringSettings|GetNumOfLights) 1))) "World") false false)
      (Variables|/Game/ModularLightSystem/Blueprints/Components/BP_Light.BP_Light_C|SetFlickerPreset (LocalVariables|GetCurrentLight) (Variables|LightStringSettings|GetFlickerPreset))
      (Variables|/Game/ModularLightSystem/Blueprints/Components/BP_Light.BP_Light_C|SetUseGradientColors? (LocalVariables|GetCurrentLight) (Variables|LightStringSettings|GetUseGradientColors?))
      (Variables|/Game/ModularLightSystem/Blueprints/Components/BP_Light.BP_Light_C|SetGradientCurve (LocalVariables|GetCurrentLight) (Variables|LightStringSettings|GetGradientCurve))
      (Variables|/Game/ModularLightSystem/Blueprints/Components/BP_Light.BP_Light_C|SetGradientForward? (LocalVariables|GetCurrentLight) (Variables|LightStringSettings|GetGradientForward?))
      (Variables|/Game/ModularLightSystem/Blueprints/Components/BP_Light.BP_Light_C|SetGradientDuration (LocalVariables|GetCurrentLight) (Variables|LightStringSettings|GetGradientDuration))
      (Utilities|Array|Add (Variables|Default|GetLights) (LocalVariables|GetCurrentLight)))))

(fn CanInteract
  (params (Caller :type Actor%20Object%20Reference))
  (return false))