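; Light trigger actor that toggles connected lights and light strings, either on overlap or as a switch with mesh, sound and interaction icon.
; Allowed classes, specific actors or the player start sequential interact messages, optionally delayed, with one-shot support.
; An in-progress lock blocks retriggering and is copied with light state to linked triggers, updating widget colors.
; The construction script sets trigger shape and, for switches, draws optional debug lines to lights.
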(event EventUpdateInteractionDisplay
  (params (Activation :type E_Show_Hide%20Enum :default "NewEnumerator0") (UseRangeIcon :type Boolean))
  ;[0.15 0.15 0.15 0.5] Interaction Icon
  (if (and UseRangeIcon (Utilities|Enum|Equal(Enum) Activation "NewEnumerator0"))
    (Rendering|SetVisibility (Variables|Default|GetWidget) true true)
    (else
      (Rendering|SetVisibility (Variables|Default|GetWidget) false true))))

(event OnComponentBeginOverlap(TriggerBox)
  (params (OverlappedComponent :type Primitive%20Component%20Object%20Reference) (OtherActor :type Actor%20Object%20Reference) (OtherComp :type Primitive%20Component%20Object%20Reference) (OtherBodyIndex :type Integer) (bFromSweep :type Boolean) (SweepResult :type Hit%20Result%20Structure%20%28by%20ref%29))
  (if (not (Variables|TriggerBoxLights|GetUseAsSwitch?))
    (CallFunction|ToggleLights OtherActor)))

(event Custom|TriggerConnectedLights
  (params (Lights :type Array%20of%20BP%20Light%20Object%20References) (Index :type Integer))
  (bind _output (Utilities|Array|Get(acopy) Lights Index))
  (bind _self self)
  (Class|BPIInteractable|CanInteract(Message) _output _self)
  (Class|BPIInteractable|Interact(Message) _output _self (not (Variables|Default|GetCurrentLightStateOn?))))

(event Custom|ToggleLights
  (params (OtherActor :type Actor%20Object%20Reference))
  (bind _connectedlights (Variables|TriggerBoxLights|GetConnectedLights))
  (bind _connectedlightstrings (Variables|TriggerBoxLights|GetConnectedLightStrings))
  (bind _array_element (Utilities|Array|ForEachLoopwithBreak (Variables|TriggerBoxLights|GetAllowOtherClasses) :!label _label)
    (:LoopBody
      (if (== (Utilities|GetClass OtherActor) _array_element)
        (goto _label Break)))
    (:Completed
      (bind _array_element_2 (Utilities|Array|ForEachLoopwithBreak (Variables|TriggerBoxLights|GetAllowSpecificActors) :!label _label_2)
        (:LoopBody
          (if (== OtherActor _array_element_2)
            (goto _label_2 Break)))
        (:Completed
          (if (Math|Boolean|ORBoolean (== (Utilities|GetClass OtherActor) _array_element) (== OtherActor _array_element_2) (and (== OtherActor (Game|GetPlayerCharacter 0)) (Variables|TriggerBoxLights|GetAllowPlayerInteraction?)))
            (if (and (Variables|TriggerBoxLights|GetDoOnce?) (not (Variables|WidgetSettings|GetAlreadyTriggered?)))
              (Variables|WidgetSettings|SetAlreadyTriggered? true)
              (Variables|Default|SetInProgress? true)
              (CallFunction|ManageConnectedTriggers)
              ;[0.03937 0.15 0.05114 0.5] For Loop with Delay (BP_Light)
              (CallFunction|TriggerConnectedLights _connectedlights (Variables|Default|GetLightIndex) :!label _label_3)
              (bind _output_get (Variables|Default|SetLightIndex (+ (Variables|Default|GetLightIndex) 1)))
              (if (Variables|TriggerBoxLights|GetTriggerWithDelay?)
                (Utilities|FlowControl|Delay (Variables|TriggerBoxLights|GetTriggerDelay)))
              (if (>= _output_get (Utilities|Array|Length _connectedlights))
                (Variables|Default|SetLightIndex 0)
                ;[0.03937 0.15 0.05114 0.5] For Loop with Delay (BP_LightString)
                (CallFunction|TriggerConnectedLightStrings _connectedlightstrings (Variables|Default|GetLightIndex) :!label _label_4)
                (bind _output_get_2 (Variables|Default|SetLightIndex (+ (Variables|Default|GetLightIndex) 1)))
                (if (Variables|TriggerBoxLights|GetTriggerWithDelay?)
                  (Utilities|FlowControl|Delay (Variables|TriggerBoxLights|GetTriggerDelay)))
                (if (>= _output_get_2 (Utilities|Array|Length _connectedlightstrings))
                  (Variables|Default|SetInProgress? false)
                  (Variables|Default|SetLightIndex 0)
                  (Variables|Default|SetCurrentLightStateOn? (not (Variables|Default|GetCurrentLightStateOn?)))
                  (CallFunction|ManageConnectedTriggers)
                  (else
                    (goto _label_4)))
                (else
                  (goto _label_3)))
              (elif (not (Variables|TriggerBoxLights|GetDoOnce?))
                (if (not (Variables|Default|GetInProgress?))
                  (Variables|Default|SetInProgress? true)
                  (CallFunction|ManageConnectedTriggers)
                  (goto _label_3))))))))))

(event Custom|TriggerConnectedLightStrings
  (params (LightStrings :type Array%20of%20BP%20Light%20String%20Object%20References) (Index :type Integer))
  (bind _output (Utilities|Array|Get(acopy) LightStrings Index))
  (bind _self self)
  (Class|BPIInteractable|CanInteract(Message) _output _self)
  (Class|BPIInteractable|Interact(Message) _output _self (not (Variables|Default|GetCurrentLightStateOn?))))

(event EventBeginPlay
  (Variables|Default|SetCurrentLightStateOn? (not (Variables|TriggerBoxLights|GetActiveStateOnEnter?)))
  (CallFunction|UpdateInteractionDisplay "NewEnumerator1" (Variables|TriggerBoxLights|GetUseInteractIcon?)))

(fn ConstructionScript
  (CallFunction|ChangeTriggerType (Variables|TriggerBoxLights|GetTriggerType))
  (Rendering|SetVisibility (Variables|Default|GetTriggerBox) (not (Variables|TriggerBoxEditor|GetHideTriggerBox)) false)
  (if (Variables|TriggerBoxLights|GetUseAsSwitch?)
    (Components|StaticMesh|SetStaticMesh (Variables|Default|GetMesh) (Variables|TriggerBoxLights|GetTriggerSwitchMesh))
    (Rendering|Material|SetMaterial (Variables|Default|GetMesh) 0 (Variables|TriggerBoxLights|GetMaterialOverride))
    (Debug|DrawConnectionLines)
    (Transformation|SetWorldScale3D (Variables|Default|GetMesh) (Variables|TriggerBoxLights|GetSwitchMeshScale))
    (Transformation|AddLocalOffset (Variables|Default|GetWidget) (Variables|TriggerBoxLights|GetInteractionIconPosition) false false)))

(fn ChangeTriggerType
  (params (Type :type E_Trigger_Type%20Enum :default "NewEnumerator0"))
  (if (Utilities|Enum|Equal(Enum) Type "NewEnumerator0")
    (Components|StaticMesh|SetStaticMesh (Variables|Default|GetTriggerBox) "/Engine/BasicShapes/Cube.Cube")
    (elif (Utilities|Enum|Equal(Enum) Type "NewEnumerator1")
      (Components|StaticMesh|SetStaticMesh (Variables|Default|GetTriggerBox) "/Engine/BasicShapes/Sphere.Sphere")
      (elif (Utilities|Enum|Equal(Enum) Type "NewEnumerator2")
        (Components|StaticMesh|SetStaticMesh (Variables|Default|GetTriggerBox) "/Engine/EngineMeshes/Cylinder.Cylinder")))))

(fn DrawConnectionLines
  (if (Variables|TriggerBoxEditor|GetShowConnectedLights)
    (for _array_element (Variables|TriggerBoxLights|GetConnectedLights)
      (Rendering|Debug|DrawDebugLine (Transformation|GetActorLocation self) (Transformation|GetActorLocation _array_element) "(R=0.297735,G=1.000000,B=0.463922,A=1.000000)" 0.0 2.0))))

(fn PlaySwitchSound
  (params (SwitchState :type Boolean))
  (bind _switchaudio (Variables|Default|GetSwitchAudio))
  (bind _switchaudio_2 (Variables|Default|GetSwitchAudio))
  (if SwitchState
    (Audio|Components|Audio|SetSound _switchaudio_2 (Variables|SwitchSounds|GetSwitchSoundOn))
    (Audio|Components|Audio|Play _switchaudio_2 0.0)
    (else
      (Audio|Components|Audio|SetSound _switchaudio (Variables|SwitchSounds|GetSwitchSoundOff))
      (Audio|Components|Audio|Play _switchaudio 0.0))))

(fn ToggleConnectedLights
  (CallFunction|PlaySwitchSound (not (Variables|Default|GetCurrentLightStateOn?)))
  (CallFunction|ToggleLights (Game|GetPlayerCharacter 0)))

(fn ManageConnectedTriggers
  (CallFunction|ManageWidgetColors)
  (for _array_element (Variables|TriggerBoxConnections|GetConnectedTriggers)
    (Variables|BP_LightSwitchTrigger_C|SetCurrentLightStateOn? _array_element (Variables|Default|GetCurrentLightStateOn?))
    (Variables|BP_LightSwitchTrigger_C|SetInProgress? _array_element (Variables|Default|GetInProgress?))
    (CallFunction|ManageWidgetColors _array_element)))

(fn ManageWidgetColors
  (bind _aswbp_light_interaction (Utilities|Casting|CastToWBP_LightInteraction (UserInterface|GetUserWidgetObject (Variables|Default|GetWidget))))
  (if (Variables|Default|GetInProgress?)
    (Appearance|SetColorandOpacity (Variables|/Game/ModularLightSystem/Widget/WBP_LightInteraction.WBP_LightInteraction_C|GetRangeIndicator _aswbp_light_interaction) (Variables|WidgetSettings|GetWidgetNotUsableColor) :!class /Script/UMG.Image)
    (else
      (Appearance|SetColorandOpacity (Variables|/Game/ModularLightSystem/Widget/WBP_LightInteraction.WBP_LightInteraction_C|GetRangeIndicator _aswbp_light_interaction) (Variables|WidgetSettings|GetWidgetUsableColor) :!class /Script/UMG.Image))))

(fn ToggleConnectedLightStrings
  (CallFunction|PlaySwitchSound (not (Variables|Default|GetCurrentLightStateOn?)))
  (CallFunction|ToggleLights (Game|GetPlayerCharacter 0)))

(fn CanInteract
  (params (Caller :type Actor%20Object%20Reference))
  (return false))