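; BP_PowerSupply is a power source that feeds voltage to chains of connected lights.
; Every tick it walks ConnectedLights: with positive ProvidedVoltage, each light recalculates its needed voltage, receives the full supplied value as input and updates its chain state.
; With no positive voltage, it deactivates each light's entire chain.
; Both passes stop at the first light not set to use a power supply.
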(event EventTick
  (params (DeltaSeconds :type Float%20%28single-precision%29))
  (CallFunction|DistributeVoltage))

(fn ConstructionScript)

(fn DistributeVoltage
  (if (> (Variables|PowerSupplySettings|GetProvidedVoltage) 0.0)
    ;[0.03289 0.2292 0 0.5] Proceed with given voltage, and check the whole light chain
    (bind _array_element (Utilities|Array|ForEachLoopwithBreak (Variables|PowerSupplySettings|GetConnectedLights) :!label _label)
      (:LoopBody
        (if (Variables|/Game/MLS/Blueprints/Components/BP_Light.BP_Light_C|GetUsePowerSupply? _array_element)
          (bind _voltage (Default|CalculateVoltageNeeded _array_element))
          (Variables|/Game/MLS/Blueprints/Components/BP_Light.BP_Light_C|SetTotalVoltageNeeded _array_element _voltage)
          (bind _output_get (Variables|/Game/MLS/Blueprints/Components/BP_Light.BP_Light_C|SetInputVoltage _array_element (Variables|PowerSupplySettings|GetProvidedVoltage)))
          (Default|SetLampChainState _array_element _output_get)
          (else
            (goto _label Break)))))
    (else
      ;[0.15 0 0 0.5] Missing voltage, disable all connected lines
      (bind _array_element_2 (Utilities|Array|ForEachLoopwithBreak (Variables|PowerSupplySettings|GetConnectedLights) :!label _label_2)
        (:LoopBody
          (if (Variables|/Game/MLS/Blueprints/Components/BP_Light.BP_Light_C|GetUsePowerSupply? _array_element_2)
            (Variables|/Game/MLS/Blueprints/Components/BP_Light.BP_Light_C|SetInputVoltage _array_element_2 (Variables|PowerSupplySettings|GetProvidedVoltage))
            (Default|DeactivateEntireChain _array_element_2)
            (else
              (goto _label_2 Break))))))))