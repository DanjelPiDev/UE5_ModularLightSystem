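; BP_SimplePlayerCharacter is a basic player-controlled character Blueprint in the MLS demo content.
; When a player controller takes control, it adds the IMC_Default mapping context through the Enhanced Input local player subsystem.
; IA_Look drives controller yaw and pitch, while IA_Move feeds movement input along the actor's forward and right vectors, with X as forward and Y as right.
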(event Input|EnhancedActionEvents|EnhancedInputActionIA_Move
  (params (ActionValue :type Vector%202D%20Structure) (ElapsedSeconds :type Float%20%28double-precision%29) (TriggeredSeconds :type Float%20%28double-precision%29) (InputAction :type Input%20Action%20Object%20Reference :default "/Game/MLS/Levels/DemoBPs/Inputs/Actions/IA_Move.IA_Move"))
  (Pawn|Input|AddMovementInput (Transformation|GetActorForwardVector) (.x ActionValue) false)
  (Pawn|Input|AddMovementInput (Transformation|GetActorRightVector) (.y ActionValue) false))

(event Input|EnhancedActionEvents|EnhancedInputActionIA_Look
  (params (ActionValue :type Vector%202D%20Structure) (ElapsedSeconds :type Float%20%28double-precision%29) (TriggeredSeconds :type Float%20%28double-precision%29) (InputAction :type Input%20Action%20Object%20Reference :default "/Game/MLS/Levels/DemoBPs/Inputs/Actions/IA_Look.IA_Look"))
  (Pawn|Input|AddControllerYawInput (.x ActionValue))
  (Pawn|Input|AddControllerPitchInput (.y ActionValue)))

(event EventControllerChanged
  (params (OldController :type Controller%20Object%20Reference) (NewController :type Controller%20Object%20Reference))
  (bind _asplayer_controller (Utilities|Casting|CastToPlayerController NewController))
  (Input|AddMappingContext (PlayerController|LocalPlayerSubsystems|GetEnhancedInputLocalPlayerSubsystem _asplayer_controller) "/Game/MLS/Levels/DemoBPs/Inputs/IMC_Default.IMC_Default" 0 "(bIgnoreAllPressedKeysUntilRelease=True,bForceImmediately=False,bNotifyUserSettings=False)"))

(fn ConstructionScript)