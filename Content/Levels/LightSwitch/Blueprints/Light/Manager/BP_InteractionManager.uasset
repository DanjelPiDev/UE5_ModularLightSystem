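; Interaction manager that lets the player use lights (BP_Light) and light switch triggers (BP_LightSwitchTrigger).
; Each Tick, a camera-forward sphere trace caches the hit actor and updates its interaction prompt.
; The IA_Use Enhanced Input action toggles a cached light through BPI_Interactable or calls ToggleConnectedLights on a switch trigger.
; Its construction script applies global show/hide flags to trigger volumes on every light and switch trigger in the level.
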(event Input|EnhancedActionEvents|EnhancedInputActionIA_Use
  (params (ActionValue :type Boolean) (ElapsedSeconds :type Float%20%28double-precision%29) (TriggeredSeconds :type Float%20%28double-precision%29) (InputAction :type Input%20Action%20Object%20Reference :default "/Game/FirstPerson/Input/Actions/IA_Use.IA_Use"))
  (bind _lasthitactor (Variables|Default|GetLastHitActor))
  ;[0.02382 0.1004 0.15 0.5] Check that the player is looking at the light switch OR is in the trigger sphere.
  (Utilities|IsValid (Variables|Default|GetLastHitActor)
    (:Is%20Valid
      (if ActionValue
        (bind _asbp_light (Utilities|Casting|CastToBP_Light _lasthitactor)
          (:then
            (if (Variables|/Game/Levels/LightSwitch/Blueprints/Light/Components/BP_Light.BP_Light_C|GetHasToLookAtSwitch? _asbp_light)
              (if (Class|KismetSystemLibrary|DoesClassImplementInterface (Utilities|GetClass _asbp_light) "/Game/Levels/LightSwitch/Blueprints/Light/Interfaces/BPI_Interactable.BPI_Interactable_C")
                (Class|BPIInteractable|Interact(Message) (stale EventTick _hitactor) self (not (Variables|/Game/Levels/LightSwitch/Blueprints/Light/Components/BP_Light.BP_Light_C|GetIsActive? _asbp_light)) :!label _label))
              (else
                ;;[0.15 0 0.1166 0.5] Approx interaction (With sphere, player does not need to look the the switch directly)
                (if (and ActionValue (not (Variables|/Game/Levels/LightSwitch/Blueprints/Light/Components/BP_Light.BP_Light_C|GetHasToLookAtSwitch? _asbp_light)))
                  (goto _label)))))
          (:CastFailed
            ;[0.15 0.15 0.15 0.5] Light Switch Logic
            (bind _asbp_light_switch_trigger (Utilities|Casting|CastToBP_LightSwitchTrigger _lasthitactor)
              (:then
                (Default|ToggleConnectedLights _asbp_light_switch_trigger))
              (:CastFailed
                (goto _label)))))))))

(event EventTick
  (params (DeltaSeconds :type Float%20%28single-precision%29))
  ;[0.02382 0.1004 0.15 0.5] Check that the player is looking at the light switch OR is in the trigger sphere.
  (bind (_didhit _hitactor) (Utilities|GetInteractableLightSwitch (Variables|InteractionManagerSettings|GetTraceRadius) (Variables|InteractionManagerSettings|GetTraceDistance) (Variables|InteractionManagerSettings|GetActorsToIgnore)))
  (if _didhit
    (bind _output_get (Variables|Default|SetLastHitActor _hitactor))
    (bind _asbp_light (Utilities|Casting|CastToBP_Light _output_get)
      (:then
        (Class|BPIInteractable|UpdateInteractionDisplay(Message) _output_get "NewEnumerator0" (Variables|/Game/Levels/LightSwitch/Blueprints/Light/Components/BP_Light.BP_Light_C|GetUseInteractIcon? _asbp_light)))
      (:CastFailed
        (bind _asbp_light_switch_trigger (Utilities|Casting|CastToBP_LightSwitchTrigger (Variables|Default|GetLastHitActor)))
        (Class|BPIInteractable|UpdateInteractionDisplay(Message) _asbp_light_switch_trigger "NewEnumerator0" (Variables|/Game/Levels/LightSwitch/Blueprints/Light/Components/BP_LightSwitchTrigger.BP_LightSwitchTrigger_C|GetUseInteractIcon? _asbp_light_switch_trigger))))
    (else
      (bind _asbp_light_2 (Utilities|Casting|CastToBP_Light (Variables|Default|GetLastHitActor))
        (:then
          (Class|BPIInteractable|UpdateInteractionDisplay(Message) (Variables|Default|GetLastHitActor) "NewEnumerator1" (Variables|/Game/Levels/LightSwitch/Blueprints/Light/Components/BP_Light.BP_Light_C|GetUseInteractIcon? _asbp_light_2)))
        (:CastFailed
          (bind _asbp_light_switch_trigger_2 (Utilities|Casting|CastToBP_LightSwitchTrigger (Variables|Default|GetLastHitActor))
            (:then
              (Class|BPIInteractable|UpdateInteractionDisplay(Message) _asbp_light_switch_trigger_2 "NewEnumerator1" (Variables|/Game/Levels/LightSwitch/Blueprints/Light/Components/BP_LightSwitchTrigger.BP_LightSwitchTrigger_C|GetUseInteractIcon? _asbp_light_switch_trigger_2)))
            (:CastFailed
              _))))
      (Variables|Default|SetLastHitActor 0))))

(event EventBeginPlay
  (bind _returnvalue (Game|GetPlayerController 0))
  ;[0.15 0.15 0.15 0.5] Init Player inputs
  (Input|EnableInput _returnvalue)
  (Input|AddMappingContext (PlayerController|LocalPlayerSubsystems|GetEnhancedInputLocalPlayerSubsystem _returnvalue) (Variables|InteractionManagerSettings|GetInputMapping) 0 "(bIgnoreAllPressedKeysUntilRelease=True,bForceImmediately=False,bNotifyUserSettings=False)"))

(fn ConstructionScript
  (CallFunction|ToggleAllLightTriggerVisibility)
  (CallFunction|ToggleAllTriggersVisibility))

(fn ToggleAllTriggersVisibility
  (bind _showalltriggers_ (Variables|InteractionManagerSettings|GetShowAllTriggers?))
  (bind _returnvalue (not _showalltriggers_))
  (bind _outactors (Actor|GetAllActorsOfClass "/Game/Levels/LightSwitch/Blueprints/Light/Components/BP_LightSwitchTrigger.BP_LightSwitchTrigger_C"))
  (for _array_element _outactors
    (Variables|/Game/Levels/LightSwitch/Blueprints/Light/Components/BP_LightSwitchTrigger.BP_LightSwitchTrigger_C|SetHideTriggerBox _array_element _returnvalue)
    (Class|PrimitiveComponent|SetVisibleinSceneCaptureOnly (Variables|/Game/Levels/LightSwitch/Blueprints/Light/Components/BP_LightSwitchTrigger.BP_LightSwitchTrigger_C|GetTriggerBox _array_element) _returnvalue)))

(fn ToggleAllLightTriggerVisibility
  (bind _showalllighttriggers_ (Variables|InteractionManagerSettings|GetShowAllLightTriggers?))
  (bind _returnvalue (not _showalllighttriggers_))
  (bind _outactors (Actor|GetAllActorsOfClass "/Game/Levels/LightSwitch/Blueprints/Light/Components/BP_Light.BP_Light_C"))
  (for _array_element _outactors
    (Variables|/Game/Levels/LightSwitch/Blueprints/Light/Components/BP_Light.BP_Light_C|SetHideTriggers _array_element _returnvalue)
    (Class|PrimitiveComponent|SetVisibleinSceneCaptureOnly (Variables|/Game/Levels/LightSwitch/Blueprints/Light/Components/BP_Light.BP_Light_C|GetTriggerInteraction _array_element) _returnvalue)))