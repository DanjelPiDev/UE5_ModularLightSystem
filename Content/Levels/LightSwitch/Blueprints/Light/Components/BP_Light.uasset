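; Configurable light actor (point, rect or spot) that the player can switch on and off and that fast-moving overlapping actors can destroy.
; The construction script applies mesh, light and trigger settings and draws circuit debug info, while destruction cascades through linked Series lights.
; Tick drives timer-randomized flicker, looping gradient color, audio and a camera-facing interaction widget.
; Toggling and gradient color act only on the point light.
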(event EventTick
  (params (DeltaSeconds :type Float%20%28single-precision%29))
  (CallFunction|InterpolateLightFlicker)
  (CallFunction|PlayLightAudio)
  (CallFunction|DoGradientLight DeltaSeconds)
  (CallFunction|SetWidgetRotation))

(event EventBeginPlay
  (CallFunction|StartLightFlicker)
  (CallFunction|UpdateInteractionDisplay "NewEnumerator1" (Variables|LightInteraction|GetAllowDirectInteraction?)))

(event EventUpdateInteractionDisplay
  (params (Activation :type E_Show_Hide%20Enum :default "NewEnumerator0") (UseRangeIcon :type Boolean))
  ;[0.15 0.15 0.15 0.5] Interaction Icon
  (if (and (and UseRangeIcon (Utilities|Enum|Equal(Enum) Activation "NewEnumerator0")) (not (Variables|LightInteraction|GetIsDestroyed?)))
    (Rendering|SetVisibility (Variables|Default|GetWidget) true true)
    (else
      (Rendering|SetVisibility (Variables|Default|GetWidget) false true))))

(event EventInteract
  (params (Caller :type Actor%20Object%20Reference) (ActiveState :type Boolean))
  ;[0.1214 0.04666 0.15 0.5] Interaction
  (if (and (or (and (Variables|LightInteraction|GetHasToLookAtSwitch?) (Variables|LightInteraction|GetIsInteractable?)) (and (not (Variables|LightInteraction|GetHasToLookAtSwitch?)) (Variables|LightInteraction|GetIsInteractable?))) (not (Variables|LightInteraction|GetIsDestroyed?)))
    (CallFunction|ToggleLight ActiveState)))

(event OnComponentBeginOverlap(TriggerInteraction)
  (params (OverlappedComponent :type Primitive%20Component%20Object%20Reference) (OtherActor :type Actor%20Object%20Reference) (OtherComp :type Primitive%20Component%20Object%20Reference) (OtherBodyIndex :type Integer) (bFromSweep :type Boolean) (SweepResult :type Hit%20Result%20Structure%20%28by%20ref%29))
  (bind _returnvalue (Game|GetPlayerCharacter 0))
  (bind _self self)
  (bind _returnvalue_2 (== OtherActor _returnvalue))
  ;[0 0.15 0.1494 0.5] Approx Trigger via Sphere (Player does not need to look at the Light)
  (if _returnvalue_2
    (if (and _returnvalue_2 (not (Variables|LightInteraction|GetHasToLookAtSwitch?)))
      (if (Class|KismetSystemLibrary|DoesClassImplementInterface (Utilities|GetClass _self) "/Game/Levels/LightSwitch/Blueprints/Light/Interfaces/BPI_Interactable.BPI_Interactable_C")
        (CallFunction|CanInteract _self))
      (else
        (Variables|LightInteraction|SetIsInteractable? false)))))

(event OnComponentBeginOverlap(TriggerLightDestruction)
  (params (OverlappedComponent :type Primitive%20Component%20Object%20Reference) (OtherActor :type Actor%20Object%20Reference) (OtherComp :type Primitive%20Component%20Object%20Reference) (OtherBodyIndex :type Integer) (bFromSweep :type Boolean) (SweepResult :type Hit%20Result%20Structure%20%28by%20ref%29))
  ;[0.15 0.1158 0 0.5] Destroy the light with a projectile (Or something else) with a defined velocity greater then the given threshold
  (if (> (Math|Vector|VectorLength (Transformation|GetVelocity OtherActor)) (Variables|LightTrigger|GetVelocityThreshold))
    (Variables|LightSettings|SetLightHealth 0.0)
    (CallFunction|DestroyLight)))

(event OnComponentEndOverlap(TriggerInteraction)
  (params (OverlappedComponent :type Primitive%20Component%20Object%20Reference) (OtherActor :type Actor%20Object%20Reference) (OtherComp :type Primitive%20Component%20Object%20Reference) (OtherBodyIndex :type Integer))
  (bind _returnvalue (Game|GetPlayerCharacter 0))
  (bind _returnvalue_2 (== OtherActor _returnvalue))
  ;[0 0.15 0.1494 0.5] Approx Trigger via Sphere (Player does not need to look at the Light)
  (if _returnvalue_2
    (if (and _returnvalue_2 (not (Variables|LightInteraction|GetHasToLookAtSwitch?)))
      (Variables|LightInteraction|SetIsInteractable? false))))

(fn ConstructionScript
  (bind _triggerinteraction (Variables|Default|GetTriggerInteraction))
  (bind _rectlight (Variables|Default|GetRectLight))
  (bind _pointlight (Variables|Components|GetPointLight))
  (bind _lighttype (Variables|LightSettings|GetLightType))
  (bind _lightsize (Variables|LightSettings|GetLightSize))
  (bind _returnvalue (Utilities|Enum|Equal(Enum) _lighttype "NewEnumerator0"))
  (bind _returnvalue_2 (Utilities|Enum|Equal(Enum) _lighttype "NewEnumerator2"))
  (bind _returnvalue_3 (Utilities|Enum|Equal(Enum) _lighttype "NewEnumerator1"))
  ;[0.15 0.15 0.15 0.5] Debug
  (Debug|ShowCircuitConnections)
  (Transformation|AddLocalOffset (Variables|Default|GetWidget) (Variables|LightInteraction|GetInteractionPosition) false false)
  ;[0.15 0.15 0.15 0.5] Check LightType
  (Rendering|SetVisibility (Variables|Components|GetPointLight) _returnvalue false)
  (Rendering|SetVisibility (Variables|Default|GetRectLight) _returnvalue_3 false)
  (Rendering|SetVisibility (Variables|Default|GetSpotLight) _returnvalue_2 false)
  (Rendering|SetVisibility (Variables|Default|GetRectLight) _returnvalue_3 false)
  (Rendering|SetVisibility (Variables|Components|GetPointLight) _returnvalue false)
  (Rendering|SetVisibility (Variables|Default|GetSpotLight) _returnvalue_2 false)
  (Rendering|SetVisibility (Variables|Default|GetSpotLight) _returnvalue_2 false)
  (Rendering|SetVisibility (Variables|Components|GetPointLight) _returnvalue false)
  (Rendering|SetVisibility (Variables|Default|GetRectLight) _returnvalue_3 false)
  (Variables|LightInteraction|SetIsActive? (Variables|LightSettings|GetDefaultOn?))
  (Variables|LightInteraction|SetIsDestroyed? (Variables|LightSettings|GetDefaultDestroyed?))
  (if (or (not (Variables|LightSettings|GetDefaultOn?)) (Variables|LightSettings|GetDefaultDestroyed?))
    (Rendering|Components|Light|SetIntensity (Variables|Components|GetPointLight) 0.0)
    (else
      (Rendering|Components|Light|SetIntensity _pointlight (Variables|LightSettings|GetLightIntensity))))
  (Rendering|Components|Light|SetLightColor 0 (Math|Conversions|ToLinearColor(Color) (Variables|LightSettings|GetLightColor)) true)
  (Transformation|SetRelativeRotation (Variables|Default|GetSpotLight) (Math|Conversions|RotationFromXVector (Variables|LightSettings|GetLightRotation)) false false)
  (Class|PointLightComponent|SetSourceRadius _pointlight (Variables|LightSettings|GetLightRadius))
  (if (Utilities|Enum|Equal(Enum) (Variables|LightSettings|GetLightType) "NewEnumerator1")
    (Class|RectLightComponent|SetSourceWidth _rectlight (Class|KismetMathLibrary|GetMin2D _lightsize))
    (Class|RectLightComponent|SetSourceHeight _rectlight (Class|KismetMathLibrary|GetMax2D _lightsize)))
  (if (Utilities|IsValid (Variables|LightMesh|GetMesh))
    (Components|StaticMesh|SetStaticMesh (Variables|Components|GetLightMesh) (Variables|LightMesh|GetMesh)))
  (Rendering|Material|SetMaterial (Variables|Components|GetLightMesh) 0 (Variables|LightMesh|GetMaterialOverride))
  (Transformation|AddLocalOffset (Variables|Components|GetPointLight) (Variables|LightSettings|GetLightPosition) false false)
  (Rendering|Components|Light|SetCastShadows (Variables|Components|GetPointLight) (Variables|LightSettings|GetLightCastShadow?))
  (Transformation|AddLocalOffset (Variables|Default|GetTriggerLightDestruction) (Variables|LightTrigger|GetLightTriggerPosition) false false)
  (Transformation|SetWorldScale3D (Variables|Default|GetTriggerLightDestruction) (Variables|LightTrigger|GetLightTriggerScale))
  (Physics|SetSimulatePhysics (Variables|Components|GetLightMesh) false)
  (Transformation|AddLocalOffset _triggerinteraction (Variables|LightInteraction|GetLightSwitchTriggerPosition) false false)
  (Transformation|SetWorldScale3D _triggerinteraction (Variables|LightInteraction|GetLightSwitchTriggerScale))
  (Class|PrimitiveComponent|SetVisibleinSceneCaptureOnly (Variables|Default|GetTriggerLightDestruction) (Variables|LightEditor|GetHideTriggers))
  (Class|PrimitiveComponent|SetVisibleinSceneCaptureOnly (Variables|Default|GetLightSwitchInteractIcon) (not (Variables|LightInteraction|GetAllowDirectInteraction?))))

(fn DestroyLight
  (bind _lightaudiofx (Variables|Default|GetLightAudioFX))
  (if (and (Variables|LightSettings|GetIsDestroyable?) (not (Variables|LightInteraction|GetIsDestroyed?)))
    (Utilities|IsValid (Variables|Components|GetPointLight)
      (:Is%20Valid
        (Rendering|Components|Light|SetIntensity (Variables|Default|GetSpotLight) 0.0)
        (Audio|Components|Audio|SetSound _lightaudiofx (Variables|LightAudio|GetLightAudioDestuction))
        (Audio|Components|Audio|Play _lightaudiofx 0.0)
        (Variables|LightInteraction|SetIsDestroyed? true)
        (switch Utilities|FlowControl|Switch|SwitchonE_Circuit_Type (Variables|LightCircuit|GetCircuitType)
          (:NewEnumerator0
            (for _array_element (Variables|LightCircuit|GetNextLights)
              (CallFunction|DestroyLight _array_element)
              (CallFunction|DestroyChain _array_element))))))))

(fn ToggleLight
  (params (ActiveState :type Boolean))
  (bind _returnvalue (not ActiveState))
  (bind _lightaudiofx (Variables|Default|GetLightAudioFX))
  (bind _lightaudiofx_2 (Variables|Default|GetLightAudioFX))
  (bind _pointlight (Variables|Components|GetPointLight))
  (if (not (Variables|LightInteraction|GetIsDestroyed?))
    (Utilities|IsValid _pointlight
      (:Is%20Valid
        (if _returnvalue
          (Rendering|Components|Light|SetIntensity _pointlight 0.0)
          (Audio|Components|Audio|SetSound _lightaudiofx (Variables|LightAudio|GetLightAudioOff))
          (Audio|Components|Audio|Play _lightaudiofx 0.0)
          (else
            (Rendering|Components|Light|SetIntensity _pointlight (Variables|LightSettings|GetLightIntensity))
            (Audio|Components|Audio|SetSound _lightaudiofx_2 (Variables|LightAudio|GetLightAudioOn))
            (Audio|Components|Audio|Play _lightaudiofx_2 0.0)))
        (Variables|LightInteraction|SetIsActive? (not _returnvalue))))))

(fn DoLightFlicker
  (bind _flickerintensityrange (Variables|LightModes|GetFlickerIntensityRange))
  (Variables|LightModes|SetTargetIntensity (Math|Random|RandomFloatinRange (Class|KismetMathLibrary|GetMin2D _flickerintensityrange) (Class|KismetMathLibrary|GetMax2D _flickerintensityrange))))

(fn StartLightFlicker
  (bind _flickerinterval (Variables|LightModes|GetFlickerInterval))
  (if (and (and (Variables|LightModes|GetUseLightFlickering?) (Variables|LightInteraction|GetIsActive?)) (not (Variables|LightInteraction|GetIsDestroyed?)))
    (Utilities|Time|SetTimerbyFunctionName 0 "DoLightFlicker" (Math|Random|RandomFloatinRange (Class|KismetMathLibrary|GetMin2D _flickerinterval) (Class|KismetMathLibrary|GetMax2D _flickerinterval)) true)))

(fn InterpolateLightFlicker
  (if (and (and (Variables|LightModes|GetUseLightFlickering?) (Variables|LightInteraction|GetIsActive?)) (not (Variables|LightInteraction|GetIsDestroyed?)))
    (if (Utilities|Enum|Equal(Enum) (Variables|LightSettings|GetLightType) "NewEnumerator0")
      ;[0.15 0.15 0.15 0.5] Point Light
      (Rendering|Components|Light|SetIntensity (Variables|Components|GetPointLight) (Math|Interpolation|FInterpTo (Variables|/Script/Engine.LightComponentBase|GetIntensity (Variables|Components|GetPointLight)) (Variables|LightModes|GetTargetIntensity) (Utilities|Time|GetWorldDeltaSeconds) (Variables|LightModes|GetFlickerInterpSpeed)))
      (elif (Utilities|Enum|Equal(Enum) (Variables|LightSettings|GetLightType) "NewEnumerator1")
        ;[0.15 0.15 0.15 0.5] Rect Light
        (Rendering|Components|Light|SetIntensity (Variables|Default|GetRectLight) (Math|Interpolation|FInterpTo (Variables|/Script/Engine.LightComponentBase|GetIntensity (Variables|Default|GetRectLight)) (Variables|LightModes|GetTargetIntensity) (Utilities|Time|GetWorldDeltaSeconds) (Variables|LightModes|GetFlickerInterpSpeed)))
        (elif (Utilities|Enum|Equal(Enum) (Variables|LightSettings|GetLightType) "NewEnumerator2")
          ;[0.15 0.15 0.15 0.5] Spot Light
          (Rendering|Components|Light|SetIntensity (Variables|Default|GetSpotLight) (Math|Interpolation|FInterpTo (Variables|/Script/Engine.LightComponentBase|GetIntensity (Variables|Default|GetSpotLight)) (Variables|LightModes|GetTargetIntensity) (Utilities|Time|GetWorldDeltaSeconds) (Variables|LightModes|GetFlickerInterpSpeed))))))))

(fn PlayLightAudio
  (bind _lightaudio (Variables|Default|GetLightAudio))
  (bind _lightaudio_2 (Variables|Default|GetLightAudio))
  (if (and (not (Variables|LightInteraction|GetIsDestroyed?)) (Variables|LightInteraction|GetIsActive?))
    (if (not (Variables|LightAudio|GetAudioIsPlaying?))
      (if (and (Variables|LightModes|GetUseLightFlickering?) (not (Variables|LightAudio|GetAudioIsPlaying?)))
        (Audio|Components|Audio|SetSound _lightaudio_2 (Variables|LightAudio|GetLightAudioFlicker))
        (Audio|Components|Audio|Play _lightaudio_2 0.0)
        (else
          (Audio|Components|Audio|SetSound _lightaudio (Variables|LightAudio|GetLightAudioGeneral))
          (Audio|Components|Audio|Play _lightaudio 0.0)))
      (Variables|LightAudio|SetAudioIsPlaying? true))
    (else
      (Audio|Components|Audio|Stop (Variables|Default|GetLightAudio))
      (Variables|LightAudio|SetAudioIsPlaying? false))))

(fn DoGradientLight
  (params (DeltaSeconds :type Float%20%28double-precision%29))
  (if (Variables|LightModes|GetUseGradientColors?)
    (if (Variables|LightModes|GetGradientForward?)
      (bind _output_get (Variables|LightModes|SetGradientElapsedTime (+ DeltaSeconds (Variables|LightModes|GetGradientElapsedTime))))
      (bind _output_get_2 (Variables|LightModes|SetGradientProgress (Math|Float|Clamp(Float) (/ _output_get (Variables|LightModes|GetGradientDuration)))))
      (Rendering|Components|Light|SetLightColor (Variables|Components|GetPointLight) (Math|Curves|GetLinearColorValue (Variables|LightModes|GetGradientCurve) _output_get_2) true)
      (if (> (Variables|LightModes|GetGradientElapsedTime) (Variables|LightModes|GetGradientDuration))
        (Variables|LightModes|SetGradientForward? (not (Variables|LightModes|GetGradientForward?)) :!label _label))
      (else
        (if (>= 0.0 (Variables|LightModes|GetGradientElapsedTime))
          (Variables|LightModes|SetGradientElapsedTime (Variables|LightModes|GetGradientDuration)))
        (bind _output_get_3 (Variables|LightModes|SetGradientElapsedTime (- (Variables|LightModes|GetGradientElapsedTime) DeltaSeconds)))
        (bind _output_get_4 (Variables|LightModes|SetGradientProgress (Math|Float|Clamp(Float) (/ _output_get_3 (Variables|LightModes|GetGradientDuration)))))
        (Rendering|Components|Light|SetLightColor (Variables|Components|GetPointLight) (Math|Curves|GetLinearColorValue (Variables|LightModes|GetGradientCurve) _output_get_4) true)
        (if (>= 0.0 (Variables|LightModes|GetGradientElapsedTime))
          (goto _label))))))

(fn SetWidgetRotation
  (bind _returnvalue (Game|GetPlayerCameraManager 0))
  (bind _widget (Variables|Default|GetWidget))
  (bind _returnvalue_2 (Transformation|GetWorldLocation _widget))
  (bind _returnvalue_3 (Camera|GetCameraLocation _returnvalue))
  (bind _returnvalue_4 (Math|Rotator|FindLookatRotation _returnvalue_2 _returnvalue_3))
  (bind (_roll _pitch _yaw) (Math|Rotator|BreakRotator _returnvalue_4))
  (if (Variables|LightInteraction|GetIsInteractable?)
    (Transformation|SetWorldRotation _widget (Math|Rotator|MakeRotator _roll _pitch _yaw) false false)))

(fn DestroyChain
  (params (Light :type BP%20Light%20Object%20Reference))
  (for _array_element (Variables|BP_Light_C|GetNextLights Light)
    (switch Utilities|FlowControl|Switch|SwitchonE_Circuit_Type (Variables|BP_Light_C|GetCircuitType _array_element)
      (:NewEnumerator0
        (Utilities|IsValid _array_element
          (:Is%20Valid
            (CallFunction|DestroyLight _array_element)))))))

(fn ShowCircuitConnections
  (bind _nextlights (Variables|LightCircuit|GetNextLights))
  (bind _returnvalue (Utilities|Array|Length _nextlights))
  (bind _returnvalue_2 (Utilities|String|ToString(Integer) _returnvalue))
  (switch Utilities|FlowControl|Switch|SwitchonE_Circuit_Type (Variables|LightCircuit|GetCircuitType)
    (:NewEnumerator0
      (bind _output_get (Variables|Debug|SetCircuitString "Series"))
      (Rendering|Debug|DrawDebugLine "0, 0, 0" "0, 0, 0" "(R=0.513040,G=0.440962,B=1.000000,A=1.000000)" 0.0 2.0))
    (:NewEnumerator1
      (bind _output_get_2 (Variables|Debug|SetCircuitString "Parallel"))
      (Rendering|Debug|DrawDebugLine "0, 0, 0" "0, 0, 0" "(R=0.258909,G=1.000000,B=0.331163,A=1.000000)" 0.0 2.0)))
  (switch Utilities|FlowControl|Switch|SwitchonE_Circuit_Type (Variables|LightCircuit|GetCircuitType)
    (:NewEnumerator0
      (Rendering|Components|TextRender|SetText (Variables|Default|GetDebugText) (Utilities|Text|ToText(String) (Utilities|String|Append (Utilities|String|Append (Utilities|String|Append _output_get " [") _returnvalue_2) " Connections]"))))
    (:NewEnumerator1
      (Rendering|Components|TextRender|SetText (Variables|Default|GetDebugText) (Utilities|Text|ToText(String) (Utilities|String|Append (Utilities|String|Append (Utilities|String|Append _output_get_2 " [") _returnvalue_2) " Connections]"))))))

(fn CanInteract
  (params (Caller :type Actor%20Object%20Reference))
  (Variables|LightInteraction|SetIsInteractable? true))