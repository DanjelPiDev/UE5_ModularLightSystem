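; BP_PowerSupply is a power source that feeds voltage to the lights connected to it.
; Every Tick it runs DistributeVoltage, which writes ProvidedVoltage into each connected light's CurrentVoltage.
; It sets a light active only when the voltage meets its requirement and both DefaultOn and IsDestroyed are true, otherwise inactive.
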(event EventTick
  (params (DeltaSeconds :type Float%20%28single-precision%29))
  (CallFunction|DistributeVoltage))

(fn ConstructionScript)

(fn DistributeVoltage
  (bind _providedvoltage (Variables|PowerSupplySettings|GetProvidedVoltage))
  (for _array_element (Variables|PowerSupplySettings|GetConnectedLights)
    (Variables|/Game/Levels/LightSwitch/Blueprints/Light/Components/BP_Light.BP_Light_C|SetCurrentVoltage _array_element _providedvoltage)
    (if (Math|Boolean|ANDBoolean (>= _providedvoltage (Variables|/Game/Levels/LightSwitch/Blueprints/Light/Components/BP_Light.BP_Light_C|GetRequiredVoltage _array_element)) (Variables|/Game/Levels/LightSwitch/Blueprints/Light/Components/BP_Light.BP_Light_C|GetDefaultOn? _array_element) (Variables|/Game/Levels/LightSwitch/Blueprints/Light/Components/BP_Light.BP_Light_C|GetIsDestroyed? _array_element))
      (Variables|/Game/Levels/LightSwitch/Blueprints/Light/Components/BP_Light.BP_Light_C|SetIsActive? _array_element true)
      (else
        (Variables|/Game/Levels/LightSwitch/Blueprints/Light/Components/BP_Light.BP_Light_C|SetIsActive? _array_element false)))))